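; BP_SimulationPlayerController is the player controller for a simulation involving items, product orders and delivery robots, setting up its main HUD on BeginPlay.
; After a tiny delay it creates WBP_MainHUD, injects the item, product order and delivery robot managers found in the level into its sub-widgets, and shows the mouse cursor.
; Product order requests from the HUD forward their recipe to the delivery robot manager's SetProductRobot.
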(event `self.ReceiveBeginPlay`
  (`KismetSystemLibrary.Delay` 0.001)
  (bind _returnvalue (`|CreateWidget` "/Game/Project/Widget/WBP_MainHUD.WBP_MainHUD_C" self))
  (bind _returnvalue_2 (`GameplayStatics.GetActorOfClass` "/Game/Project/Blueprint/BP_ItemManageActor.BP_ItemManageActor_C"))
  (set `ItemManagementWidget.ItemManager` _returnvalue_2 (`/Game/Project/Widget/WBP_MainHUD.WBP_ItemManagementWidget` _returnvalue))
  (bind _returnvalue_3 (`GameplayStatics.GetActorOfClass` "/Game/Project/Manager/BP_ProductOrderManager.BP_ProductOrderManager_C"))
  (bind _wbp_productordermanagementwidget (`/Game/Project/Widget/WBP_MainHUD.WBP_ProductOrderManagementWidget` _returnvalue))
  (set `ProductOrderManagementWidget.ProductManager` _returnvalue_3 _wbp_productordermanagementwidget)
  (bind _returnvalue_4 (`GameplayStatics.GetActorOfClass` "/Game/Project/Manager/BP_DeliveryRobotManager.BP_DeliveryRobotManager_C"))
  (set `ProcessProgressWidget.RobotManager` _returnvalue_4 (`/Game/Project/Widget/WBP_MainHUD.WBP_ProcessProgressWidget` _returnvalue))
  (add `ProductOrderManagementWidget.OnProductOrderRequested` _wbp_productordermanagementwidget (delegate `CustomEvent`))
  (`UserWidget.AddToViewport` _returnvalue 0)
  (set `PlayerController.bShowMouseCursor` true (`GameplayStatics.GetPlayerController` 0)))

(event `CustomEvent`
  (params (ProductRecipe :type "ProductRecipeDataAsset Object Reference"))
  (bind _returnvalue (`GameplayStatics.GetActorOfClass` "/Game/Project/Manager/BP_DeliveryRobotManager.BP_DeliveryRobotManager_C"))
  (`DeliveryRobotManager.SetProductRobot` _returnvalue ProductRecipe))

(fn `UserConstructionScript`)