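; Conveyor belt actor that detects BP_Item actors entering and leaving its start and end collision boxes.
; An item entering the start box is passed to SplineSetting, then to ItemSetting unless its state is Grabed.
; Overlap events on both boxes set and clear StartTriggered and EndTriggered, without counting overlapping items.
; The graph has no Tick logic, and both setting functions are defined outside this file.
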(event `self.StartCollisionBox.OnComponentBeginOverlap`
  (params (OverlappedComponent :type "PrimitiveComponent Object Reference") (OtherActor :type "Actor Object Reference") (OtherComp :type "PrimitiveComponent Object Reference") (OtherBodyIndex :type Integer) (bFromSweep :type Boolean) (SweepResult :type "HitResult Structure (by ref)"))
  (bind _asbp_item (cast `/Game/Project/Blueprint/BP_Item` OtherActor))
  (set `self.bStartTriggered` true)
  (`self.SplineSetting` _asbp_item)
  (if (not (`|EnumEquality` (`Item.ItemState` _asbp_item) "Grabed"))
    (`self.ItemSetting` _asbp_item)))

(event `self.StartCollisionBox.OnComponentEndOverlap`
  (params (OverlappedComponent :type "PrimitiveComponent Object Reference") (OtherActor :type "Actor Object Reference") (OtherComp :type "PrimitiveComponent Object Reference") (OtherBodyIndex :type Integer))
  (cast `/Game/Project/Blueprint/BP_Item` OtherActor)
  (set `self.bStartTriggered` false))

(event `self.EndCollisionBox.OnComponentBeginOverlap`
  (params (OverlappedComponent :type "PrimitiveComponent Object Reference") (OtherActor :type "Actor Object Reference") (OtherComp :type "PrimitiveComponent Object Reference") (OtherBodyIndex :type Integer) (bFromSweep :type Boolean) (SweepResult :type "HitResult Structure (by ref)"))
  (cast `/Game/Project/Blueprint/BP_Item` OtherActor)
  (set `self.bEndTriggered` true))

(event `self.EndCollisionBox.OnComponentEndOverlap`
  (params (OverlappedComponent :type "PrimitiveComponent Object Reference") (OtherActor :type "Actor Object Reference") (OtherComp :type "PrimitiveComponent Object Reference") (OtherBodyIndex :type Integer))
  (cast `/Game/Project/Blueprint/BP_Item` OtherActor)
  (set `self.bEndTriggered` false))

(fn `UserConstructionScript`)