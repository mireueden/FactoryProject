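; BP_RobotArm is a robot arm actor that turns its stand and checks items entering its check box.
; RobotStandRotate stores a target yaw and enables rotation, which Tick then eases toward with RInterpTo, reading world rotation but setting relative.
; The rotating flag is never cleared here.
; Overlapping BP_Item actors trigger a debug print and are passed to CheckItem, which is defined outside these graphs.
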(event `self.ReceiveBeginPlay`)

(event `self.ReceiveTick`
  (params (DeltaSeconds :type "Float (single-precision)"))
  (if (`self.bIsRotating`)
    (`SceneComponent.K2_SetRelativeRotation` (`self.RobotStandComp`) (`KismetMathLibrary.RInterpTo` (`SceneComponent.K2_GetComponentRotation` (`self.RobotStandComp`)) (`self.SettingRotator`) DeltaSeconds 1.6) false false)))

(event `self.CheckBox.OnComponentBeginOverlap`
  (params (OverlappedComponent :type "PrimitiveComponent Object Reference") (OtherActor :type "Actor Object Reference") (OtherComp :type "PrimitiveComponent Object Reference") (OtherBodyIndex :type Integer) (bFromSweep :type Boolean) (SweepResult :type "HitResult Structure (by ref)"))
  (bind _asbp_item (cast `/Game/Project/Blueprint/BP_Item` OtherActor))
  (`KismetSystemLibrary.PrintString` "Hello")
  (`self.CheckItem` _asbp_item))

(fn `RobotStandRotate`
  (params (RotateValue :type "Float (double-precision)"))
  (set `self.SettingRotator` (`KismetMathLibrary.MakeRotator` 0.0 0.0 RotateValue))
  (set `self.bIsRotating` true)
  (return))

(fn `UserConstructionScript`)